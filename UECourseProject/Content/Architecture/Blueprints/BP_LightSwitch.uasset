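; BP_LightSwitch is a light switch that turns a set of connected lights on and off when used.
; The Use event flips IsOn and sets LightIntensity to either zero or a fixed brightness.
; It then loops over ConnectedLights and applies that intensity to each one's light component, with no logic on BeginPlay, Tick or construction.
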(event EventBeginPlay)

(event Collision|EventActorBeginOverlap
  (params (OtherActor :type Actor%20Object%20Reference)))

(event EventTick
  (params (DeltaSeconds :type Float%20%28single-precision%29)))

(event EventUse
  (if (Variables|Default|GetIsOn)
    (Variables|Default|SetLightIntensity 0.0)
    (Variables|Default|SetIsOn false)
    (else
      (Variables|Default|SetLightIntensity 8.0)
      (Variables|Default|SetIsOn true)))
  (for _array_element (Variables|Default|GetConnectedLights)
    (Rendering|Components|Light|SetIntensity (Variables|/Script/Engine.Light|GetLightComponent _array_element) (Variables|Default|GetLightIntensity))))

(fn ConstructionScript)