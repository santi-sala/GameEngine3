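; BP_LightSensor is an occupancy-style light switch that toggles its Lights as pawns enter and leave its Triggers.
; BeginPlay binds every trigger's overlap events; a pawn entering shows each light component.
; On exit, CheckTriggersForPawns scans the triggers, and a false result hides the lights if the leaving actor is a pawn.
; That check only ever assigns IsPawnFound false, even on finding a pawn, so it never reports occupancy by itself.
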(event Custom|LightOnWhenBegginOverlap
  (params (OverlappedActor :type Actor%20Object%20Reference) (OtherActor :type Actor%20Object%20Reference))
  (Utilities|Casting|CastToPawn OtherActor)
  (CallFunction|SetLightsonOff true))

(event Custom|LightOffWhenEndOverlap
  (params (OverlappedActor :type Actor%20Object%20Reference) (OtherActor :type Actor%20Object%20Reference))
  (bind _istriggered (CallFunction|CheckTriggersforPawns))
  (if (not _istriggered)
    (Utilities|Casting|CastToPawn OtherActor)
    (CallFunction|SetLightsonOff false)))

(event EventBeginPlay
  (for _array_element (Variables|Default|GetTriggers)
    (Collision|BindEventtoOnActorBeginOverlap _array_element (delegate Custom|LightOnWhenBegginOverlap))
    (Collision|BindEventtoOnActorEndOverlap _array_element (delegate Custom|LightOffWhenEndOverlap))))

(fn ConstructionScript)

(fn CheckTriggersforPawns
  (bind _array_element (Utilities|Array|ForEachLoopwithBreak (Variables|Default|GetTriggers) :!label _label)
    (:LoopBody
      (if (!= (Utilities|Array|Length (Collision|GetOverlappingActors _array_element "/Script/Engine.Pawn" :!class /Script/Engine.Actor)) 0)
        (LocalVariables|SetIsPawnFound false)
        (goto _label Break)))
    (:Completed
      (return (LocalVariables|GetIsPawnFound)))))

(fn SetLightsonOff
  (params (IsSetOn :type Boolean))
  (for _array_element (Variables|Default|GetLights)
    (Rendering|SetVisibility (Variables|/Script/Engine.Light|GetLightComponent _array_element) IsSetOn false)))